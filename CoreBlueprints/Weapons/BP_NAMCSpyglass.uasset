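; Spyglass weapon that gives its holder adjustable targeting zoom and a toggleable target lock.
; After a short BeginPlay delay it enables input for the local controller, while the authority adds Buff_NAMCSpyglass to the player and removes it on EndPlay.
; The mouse wheel steps OverrideTargetingFOV within bounds while aiming or riding.
; Fire input calls ToggleUILock, which forwards to the buff's target lock when the buff reference is valid.
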(event `self.ReceiveBeginPlay`
  (`KismetSystemLibrary.Delay` 0.2)
  (bind _returnvalue (`self.GetOwnerController`))
  (`|ExecutionSequence`
    (:`then_0`
      (if (`Controller.IsLocalController` _returnvalue)
        (`self.EnableInput` _returnvalue)))
    (:`then_1`
      (`/Engine/EditorBlueprintResources/ActorMacros.Switch Has Authority`
        (:`Authority`
          (bind _asshooterplayercontroller (cast `ShooterPlayerController` _returnvalue))
          (bind _returnvalue_2 (`PrimalBuff.StaticAddBuff` "/Game/Mods/NAMC/CoreBlueprints/Buffs/Buff_NAMCSpyglass.Buff_NAMCSpyglass_C" (`ShooterPlayerController.GetPlayerCharacter` _asshooterplayercontroller)))
          (bind _asbuff_namcspyglass_c (cast `/Game/Mods/NAMC/CoreBlueprints/Buffs/Buff_NAMCSpyglass` _returnvalue_2))
          (set `self.BuffRef` _asbuff_namcspyglass_c))))))

(event `self.ReceiveEndPlay`
  (params (EndPlayReason :type "EngineTypes.EEndPlayReason Enum" :default "ActorDestroyed"))
  (bind _buffref (`self.BuffRef`))
  (`/Engine/EditorBlueprintResources/ActorMacros.Switch Has Authority`
    (:`Authority`
      (`/Engine/EditorBlueprintResources/StandardMacros.IsValid` _buffref
        (:`Is Valid`
          (`/Game/Mods/NAMC/CoreBlueprints/Buffs/Buff_NAMCSpyglass.RemoveBuff` _buffref))))))

(event `InputAction|Targeting` :consume false :overrideparent false
  (:`Pressed`
    (set `self.IsRightMouseDown` true :!label _label))
  (:`Released`
    (set `self.IsRightMouseDown` false :!label _label_2)))

(event `InputAction|GamepadLeftFire` :consume false :overrideparent false
  (:`Pressed`
    (goto _label))
  (:`Released`
    (goto _label_2)))

(event `Key|MouseScrollUp` :consume false :overrideparent false
  (bind _overridetargetingfov (`self.OverrideTargetingFOV`))
  (:`Pressed`
    (bind _asshootercharacter (cast `ShooterCharacter` (`self.GetOwner`)))
    (if (`ShooterCharacter.bIsRiding` _asshootercharacter)
      (if (> _overridetargetingfov 10.0) :!label _label_3
        (set `self.OverrideTargetingFOV` (- _overridetargetingfov 5.0)))
      (elif (`self.IsRightMouseDown`)
        (goto _label_3)))))

(event `Key|MouseScrollDown` :consume false :overrideparent false
  (bind _overridetargetingfov (`self.OverrideTargetingFOV`))
  (:`Pressed`
    (bind _asshootercharacter (cast `ShooterCharacter` (`self.GetOwner`)))
    (if (`ShooterCharacter.bIsRiding` _asshootercharacter)
      (if (< _overridetargetingfov 90.0) :!label _label_4
        (set `self.OverrideTargetingFOV` (+ _overridetargetingfov 5.0)))
      (elif (`self.IsRightMouseDown`)
        (goto _label_4)))))

(event `InputAction|Fire`
  (:`Pressed`
    (`self.ToggleUILock` :!label _label_5)))

(event `InputAction|GamepadRightFire`
  (:`Pressed`
    (goto _label_5)))

(event `ToggleUILock`
  (bind _buffref (`self.BuffRef`))
  (`/Engine/EditorBlueprintResources/StandardMacros.IsValid` _buffref
    (:`Is Valid`
      (`/Game/Mods/NAMC/CoreBlueprints/Buffs/Buff_NAMCSpyglass.ToggleTargetLock` _buffref))))

(fn `UserConstructionScript`
  (`parent.UserConstructionScript`))
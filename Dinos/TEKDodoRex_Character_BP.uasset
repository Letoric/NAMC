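; TEK DodoRex boss dino for AccessibleTEK that rewards nearby players on death with Element, Black Pearls and, unless the fight was cheesed, a TEK engram unlock buff.
; INI options cap count, level and lifetime, and extras spawned too close self-destruct.
; Timers apply Intimidated to nearby dinos and remove the boss on expiry or prolonged submersion in stasis.
; Stasis restores health, unstasis restarts the countdown, and a floating HUD shows remaining time.
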(event `Scan and Apply Intimidated Buff`
  ;[255 0 0] Apply Intimidated Buff
  (bind _returnvalue (`VictoryCore.ServerOctreeOverlapActors` (`self.K2_GetWorld` self) (`self.K2_GetActorLocation` self) 9000.0 "DINOPAWNS"))
  (for _array_element _returnvalue
    (bind _asprimaldinocharacter (cast `PrimalDinoCharacter` _array_element))
    (`PrimalBuff.StaticAddBuff` "/Game/Mods/NAMC/CoreBlueprints/Buffs/Buff_Intimidated_NAMC.Buff_Intimidated_NAMC_C" _asprimaldinocharacter null self (and (`PrimalDinoCharacter.BPIsTamed` _asprimaldinocharacter) (`PrimalCharacter.bIsFlyerDino` _asprimaldinocharacter)))))

(event `HidingUnderwater`
  (bind _underwatercount (`self.UnderwaterCount`))
  ;[0 0.9354 1] Purge if in stasis and under water for x time
  (if (`self.bStasised`)
    (bind _returnvalue (`SceneComponent.GetWorldLocation` (`self.StaticMesh1`)))
    (bind _returnvalue_2 (`BiomeZoneVolume.IsPointUnderwater` (`self.K2_GetWorld` self) _returnvalue true 0.0))
    (if _returnvalue_2
      (set `self.UnderwaterCount` (+ 1 _underwatercount))
      (if (>= _underwatercount (`self.UnderwaterCountMax`))
        (`self.K2_DestroyActor`)
        (else
          (`KismetSystemLibrary.K2_SetTimer` null "HidingUnderwater" 15.0)))
      (else
        (set `self.UnderwaterCount` 0)
        (`KismetSystemLibrary.K2_SetTimer` null "HidingUnderwater" 15.0)))))

(event `self.BPPlayDying`
  (params (KillingDamage :type "Float (single-precision)") (DamageEvent :type "EngineTypes.DamageEvent Structure (by ref)") (InstigatingPawn :type "Pawn Object Reference") (DamageCauser :type "Actor Object Reference"))
  (bind _bonusitems (`self.BonusItems`))
  ;[0 200 67.89 50] Give Rewards for non cheaters
  (if (!= DamageCauser null)
    (set `self.CheesedIt` false)
    (else
      (set `self.CheesedIt` true)))
  (bind _returnvalue (`VictoryCore.ServerOctreeOverlapActors` (`self.K2_GetWorld`) (`self.K2_GetActorLocation`) (`self.DeathGiveItemRange`) "PLAYERPAWNS"))
  (for _array_element _returnvalue
    (bind _asshootercharacter (cast `ShooterCharacter` _array_element))
    (bind _myinventorycomponent (`PrimalCharacter.MyInventoryComponent` _asshootercharacter))
    (`PrimalInventoryComponent.BPIncrementItemTemplateQuantity` _myinventorycomponent "/Game/PrimalEarth/CoreBlueprints/Resources/PrimalItemResource_Element.PrimalItemResource_Element_C" _bonusitems true false true false false false null false)
    (`PrimalInventoryComponent.BPIncrementItemTemplateQuantity` _myinventorycomponent "/Game/PrimalEarth/CoreBlueprints/Resources/PrimalItemResource_BlackPearl.PrimalItemResource_BlackPearl_C" _bonusitems true false true false false false null false)
    (if (not (`self.CheesedIt`))
      (bind _returnvalue_2 (`PrimalCharacter.HasBuff` _asshootercharacter "/Game/Mods/NAMC/CoreBlueprints/Buffs/Buff_UnlockTEKEngrams.Buff_UnlockTEKEngrams_C" false))
      (if (not _returnvalue_2)
        (`PrimalBuff.StaticAddBuff` "/Game/Mods/NAMC/CoreBlueprints/Buffs/Buff_UnlockTEKEngrams.Buff_UnlockTEKEngrams_C" _asshootercharacter))
      (else
        (bind _returnvalue_3 (`self.GetOwnerController` _asshootercharacter))
        (bind _asshooterplayercontroller (cast `ShooterPlayerController` _returnvalue_3))
        (`ShooterPlayerController.ClientServerNotification` _asshooterplayercontroller "You wanted TEK unlocked but cheesed the fight! Try again." (struct :`A` 1.0) 0.0 20.0 null null)))))

(event `self.BPTriggerStasisEvent`
  (bind _mycharacterstatuscomponent (`self.MyCharacterStatusComponent`))
  ;[0.2594 0.9713 1] Trigger underwater check from entering stasis
  (`KismetSystemLibrary.K2_SetTimer` null "HidingUnderwater" 60.0)
  (`PrimalCharacterStatusComponent.BPDirectSetCurrentStatusValue` _mycharacterstatuscomponent "Health" (`PrimalCharacterStatusComponent.BPGetMaxStatusValue` _mycharacterstatuscomponent "Health")))

(event `self.ReceiveBeginPlay`
  (`KismetSystemLibrary.Delay` 0.2)
  (`|ExecutionSequence`
    (:`then_0`
      (`/Engine/EditorBlueprintResources/ActorMacros.SwitchNetAuthority`
        (:`DedicatedServer`
          _)
        (:`PlayerServer`
          _))
      (bind _asshootergamemode (cast `ShooterGameMode` (`GameplayStatics.GetGameMode`)))
      (`|ExecutionSequence`
        (:`then_0`
          ;[1 1 1] Set INI Values and Destroy Actor if it exceeds configured max level
          (bind _returnvalue (`ShooterGameMode.GetIntOptionIni` _asshootergamemode "AccessibleTEK" "MaxDodoRexLVL"))
          (if (> _returnvalue 0)
            (bind _difficultyvalue (`ShooterGameMode.DifficultyValue` _asshootergamemode))
            (bind _returnvalue_2 (`KismetMathLibrary.FFloor` _difficultyvalue))
            (if (< _returnvalue _returnvalue_2)
              (set `self.TEKDodoRex-MaxLVL` _returnvalue_2)
              (else
                (bind _returnvalue_3 (`KismetMathLibrary.FFloor` (* _difficultyvalue 30.0)))
                (if (< _returnvalue _returnvalue_3)
                  (set `self.TEKDodoRex-MaxLVL` _returnvalue)
                  (else
                    (set `self.TEKDodoRex-MaxLVL` _returnvalue_3)))))
            (else
              (set `self.TEKDodoRex-MaxLVL` _returnvalue_3)))
          (bind _returnvalue_4 (`VictoryCore.ServerOctreeOverlapActorsClass` (`self.K2_GetWorld` self) (`self.K2_GetActorLocation` self) 100000.0 "DINOPAWNS" "TEKDodoRex_Character_BP_C"))
          (if (or (> (`KismetArrayLibrary.Array_Length` _returnvalue_4) 1) (> (`PrimalCharacterStatusComponent.BaseCharacterLevel` (`self.MyCharacterStatusComponent`)) (`self.TEKDodoRex-MaxLVL`)))
            (`self.K2_DestroyActor` self)))
        (:`then_1`
          ;[0.3986 0.5287 1] Set bonus item quantity based on dino level
          (for _array_element (`ShooterGameMode.HarvestResourceItemAmountClassMultipliers` _asshootergamemode)
            (if (`KismetStringLibrary.EqualEqual_StrStr` (break `ShooterGameMode.ClassMultiplier` _array_element) "Element")
              (set `self.BonusItems` (* (`KismetMathLibrary.FFloor` (`.Multiplier` (break `ShooterGameMode.ClassMultiplier` _array_element))) (* (+ (/ (`PrimalCharacterStatusComponent.BaseCharacterLevel` (`self.MyCharacterStatusComponent`)) (`KismetMathLibrary.FFloor` (`ShooterGameMode.DifficultyValue` _asshootergamemode))) 20) (`KismetMathLibrary.FFloor` (`ShooterGameMode.HarvestAmountMultiplier` _asshootergamemode)))))
              (break)))
          (`KismetSystemLibrary.K2_SetTimer` null "Scan and Apply Intimidated Buff" 5.0 true))))
    (:`then_1`
      ;[0.8156 1 0] Set initial disappear time and monitor time then destroy actor at defined time
      (set `self.DisappearTimeInSeconds` (- (`KismetSystemLibrary.GetGameTimeInSeconds`) (`KismetMathLibrary.Conv_FloatToDouble` (* (`self.DisappearInTime_Duration`) -1.0))) false)
      (`/Engine/EditorBlueprintResources/ActorMacros.Switch Has Authority`
        (:`Authority`
          (`KismetSystemLibrary.K2_SetTimerDelegate` (delegate `Check for Expiration`) 15.0 true))))))

(event `Check for Expiration`
  (bind (_returnvalue_x _returnvalue_y _returnvalue_z) (`KismetMathLibrary.BreakVector` (`self.K2_GetActorLocation`)))
  (bind _returnvalue (`KismetMathLibrary.Conv_DoubleToFloat` (- (`self.DisappearTimeInSeconds`) (`KismetSystemLibrary.GetGameTimeInSeconds`))))
  ;[0.8156 1 0] Set initial disappear time and monitor time then destroy actor at defined time
  (if (`self.bStasised`)
    (`KismetSystemLibrary.K2_SetTimer` null "HidingUnderwater" 15.0 :!label _label)
    (elif (> _returnvalue 0.0)
      (`self.Debug` (`KismetStringLibrary.Concat_StrStr` (`KismetStringLibrary.Conv_DoubleToString` _returnvalue) " seconds left on timer") false false true 3.0)
      (goto _label)
      (else
        (bind _returnvalue_2 (`VictoryCore.ServerOctreeOverlapActors` (`self.K2_GetWorld`) (`KismetMathLibrary.MakeVector` _returnvalue_x _returnvalue_y _returnvalue_z) 30000.0 "PLAYERPAWNS"))
        (set `self.PlayersNearDodoRexInt` (`KismetArrayLibrary.Array_Length` _returnvalue_2))
        (`self.Debug` (`KismetTextLibrary.Conv_TextToString` (`|FormatText` "Destroyed DodoRex at X:{X} Y:{Y} Z:{Z} with {time} left on timer. Players nearby: {players}" (`KismetTextLibrary.Conv_DoubleToText` _returnvalue_x "HalfToEven" false 1 324 0 0) (`KismetTextLibrary.Conv_DoubleToText` _returnvalue_y "HalfToEven" false 1 324 0 0) (`KismetTextLibrary.Conv_DoubleToText` _returnvalue_z "HalfToEven" false 1 324 0 0) (`KismetTextLibrary.Conv_DoubleToText` 0.0 "HalfToEven" false 1 324 0 0) (`KismetTextLibrary.Conv_IntToText` (`self.PlayersNearDodoRexInt`) false))) false false true 3.0)
        (`self.K2_DestroyActor`)))))

(event `self.BlueprintDrawFloatingHUD`
  (params (HUD :type "ShooterHUD Object Reference") (CenterX :type "Float (single-precision)") (CenterY :type "Float (single-precision)") (DrawScale :type "Float (single-precision)"))
  (bind _returnvalue (* DrawScale 3.0))
  ;[1 1 1] Draw HUD with timer countdown
  (`Canvas.BPDrawTextCentered` (`HUD.Canvas` HUD) "/Game/OldAssets/UI/HUD/Roboto18.Roboto18" (`KismetTextLibrary.Conv_TextToString` (`|FormatText` "Remaining Time: {Test}" (`KismetTextLibrary.Conv_StringToText` (`KismetStringLibrary.Conv_IntToString` (`KismetMathLibrary.FFloor` (`KismetMathLibrary.Conv_DoubleToFloat` (- (`self.DisappearTimeInSeconds`) (`KismetSystemLibrary.GetGameTimeInSeconds`)))))))) CenterX CenterY _returnvalue _returnvalue true true))

(fn `BPUnstasis`
  (set `self.DisappearTimeInSeconds` (- (`KismetSystemLibrary.GetGameTimeInSeconds`) (`KismetMathLibrary.Conv_FloatToDouble` (* (`self.DisappearInTime_Duration`) -1.0))) true))

(fn `Debug`
  (params (`Message Text` :type String) (PrintString :type Boolean) (Notification :type Boolean) (toServerLog :type Boolean) (DisplayTime :type "Float (double-precision)"))
  (bind _returnvalue (`GameplayStatics.GetGameMode`))
  (bind _returnvalue_2 (`KismetStringLibrary.Concat_StrStr` (`KismetMathLibrary.SelectString` "AccessibleTEK: Server: " "AccessibleTEK: Client: " (`self.HasAuthority`)) `Message Text`))
  (if PrintString
    (`KismetSystemLibrary.PrintString` _returnvalue_2))
  (`/Engine/EditorBlueprintResources/StandardMacros.IsValid` _returnvalue
    (:`Is Valid`
      (bind _asshootergamemode (cast `ShooterGameMode` _returnvalue))
      (if Notification
        (`|ExecutionSequence`
          (:`then_0`
            (`ShooterGameMode.SendServerNotification` _asshootergamemode _returnvalue_2 (struct :`R` 0.341845 :`G` 1.0 :`B` 0.32 :`A` 1.0) 1.0 DisplayTime null null -1 -1 false))
          (:`then_1`
            (if toServerLog :!label _label
              (`ShooterGameMode.PrintToServerGameLog` _asshootergamemode _returnvalue_2 true))))
        (else
          (goto _label))))
    (:`Is Not Valid`
      (bind _asshooterplayercontroller (cast `ShooterPlayerController` (`GameplayStatics.GetPlayerController` 0))
        (:`then`
          (`ShooterPlayerController.ClientServerNotification` _asshooterplayercontroller _returnvalue_2 (struct :`R` 1.0 :`A` 1.0) 1.0 DisplayTime null null))
        (:`CastFailed`
          (`KismetSystemLibrary.PrintString` "Controller Cast failed"))))))

(fn `UserConstructionScript`
  (`parent.UserConstructionScript`)
  (bind _asshootergamemode (cast `ShooterGameMode` (`GameplayStatics.GetGameMode`)))
  (`|ExecutionSequence`
    (:`then_0`
      (bind _returnvalue (`ShooterGameMode.GetIntOptionIni` _asshootergamemode "AccessibleTEK" "MaxDodoRexCount"))
      (set `self.TEKDodoRex-Count` (`KismetMathLibrary.SelectInt` _returnvalue (`self.TEKDodoRex-Count`) (> _returnvalue 0)))
      (bind _outactors (`GameplayStatics.GetAllActorsOfClass` "TEKDodoRex_Character_BP_C"))
      (if (> (`KismetArrayLibrary.Array_Length` _outactors) (`self.TEKDodoRex-Count`))
        (`self.K2_DestroyActor` self :!label _label)
        (else
          (bind _returnvalue_2 (`VictoryCore.ServerOctreeOverlapActorsClass` (`self.K2_GetWorld` self) (`self.K2_GetActorLocation` self) 100000.0 "DINOPAWNS" "TEKDodoRex_Character_BP_C"))
          (if (> (`KismetArrayLibrary.Array_Length` _returnvalue_2) 1)
            (goto _label)))))
    (:`then_1`
      (bind _returnvalue_3 (`ShooterGameMode.GetFloatOptionIni` _asshootergamemode "AccessibleTEK" "DisappearTimeInSeconds"))
      (set `self.DisappearInTime_Duration` (`KismetMathLibrary.SelectFloat` _returnvalue_3 (`self.DisappearInTime_Duration`) (> _returnvalue_3 0.0))))))
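; ImpLystro dino character Blueprint: a pettable Lystro variant with wild population culling and element dust conversion.
; Construction reads the INI wild cap and gathers nearby same-class dinos, which a server Purge timer trims by destroying stasised untamed ones.
; ConvertElement reschedules itself, turning inventory dust into shards.
; BeginPlay applies an INI name override, and the team-only "Pet It" entry adds an XP buff and plays montages.
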(event Custom|Purge
  (bind _wildinarea (Variables|Default|GetWildinArea))
  (bind _item (Utilities|Array|Get(acopy) _wildinarea))
  (if (> (Utilities|Array|Length _wildinarea) (Math|Integer|Min(Integer) (/ (Variables|Default|GetMaxWildCount) 5) 1))
    (bind _asimplystro_character_bp_c (Utilities|Casting|CastToImpLystro_Character_BP _item)
      (:then
        (if (and (not (Class|PrimalDinoCharacter|BPIsTamed _asimplystro_character_bp_c)) (Variables|/Script/Engine.Actor|GetbStasised _asimplystro_character_bp_c))
          (Utilities|IsValid _item
            (:Is%20Valid
              (Class|VictoryCore|RemoveActorfromCustomActorList (Class|Actor|GetWorld) "ImpLystro" _asimplystro_character_bp_c)
              (Actor|DestroyActor _item))
            (:Is%20Not%20Valid
              (Class|VictoryCore|RemoveActorfromCustomActorList (Class|Actor|GetWorld) "ImpLystro")))))
      (:CastFailed
        _))
    (Utilities|Array|RemoveIndex _wildinarea)
    (Utilities|Time|SetTimerbyFunctionName 0 "Purge" 2.0)
    (else
      (Utilities|Time|ClearTimerbyFunctionName 0 "Purge"))))

(event Custom|ConvertElement
  (bind _myinventorycomponent (Variables|Default|GetMyInventoryComponent))
  (bind _dustconvertamount (Variables|Default|GetDustConvertAmount))
  (bind _dustconvertchecktime (Variables|Default|GetDustConvertCheckTime))
  (bind _returnvalue (Class|PrimalInventoryComponent|GetItemTemplateQuantity _myinventorycomponent "/Game/Extinction/CoreBlueprints/Resources/PrimalItemResource_ElementDust.PrimalItemResource_ElementDust_C" 0 true false false false))
  (if (>= _returnvalue _dustconvertamount)
    (Class|PrimalInventoryComponent|BPGetItemOfTemplate _myinventorycomponent "/Game/Extinction/CoreBlueprints/Resources/PrimalItemResource_ElementDust.PrimalItemResource_ElementDust_C" true false false false false false false false false false)
    (Class|PrimalInventoryComponent|BPIncrementItemTemplateQuantity _myinventorycomponent "/Game/Extinction/CoreBlueprints/Resources/PrimalItemResource_ElementDust.PrimalItemResource_ElementDust_C" (* _dustconvertamount -1) true false false false false false 0 false)
    (Class|PrimalInventoryComponent|BPIncrementItemTemplateQuantity _myinventorycomponent "/Game/PrimalEarth/CoreBlueprints/Resources/PrimalItemResource_ElementShard.PrimalItemResource_ElementShard_C" (/ _dustconvertamount 10) true false false false false false 0 false)
    (Utilities|Time|SetTimerbyFunctionName 0 "ConvertElement" 1.0)
    (else
      (Utilities|Time|SetTimerbyFunctionName 0 "ConvertElement" (Math|Random|RandomFloatinRange (/ _dustconvertchecktime 1.2) (* _dustconvertchecktime 1.2))))))

(event EventBeginPlay
  (Utilities|FlowControl|Delay 0.2)
  (Networking|SwitchHasAuthority
    (:Authority
      (Utilities|FlowControl|Sequence
        (:then_0
          (Utilities|Time|SetTimerbyFunctionName 0 "Purge" 0.5))
        (:then_1
          (bind _asshootergamemode (Utilities|Casting|CastToShooterGameMode (Game|GetGameMode)))
          (bind _returnvalue (Class|ShooterGameMode|GetStringOption _asshootergamemode "ImpLystro" "DinoName"))
          (if (not (Utilities|Enum|Equal(Enum) _returnvalue ""))
            (Variables|Default|SetDinoName _returnvalue true)
            (Variables|Default|SetDescriptiveName (Variables|Default|GetDinoName) :!label _label)
            (Development|PrintString (Variables|Default|GetDinoName))))))
    (:Remote
      (Utilities|FlowControl|Delay 0.2)
      (goto _label))))

(event EventEndPlay
  (params (EndPlayReason :type EEndPlayReason%20Enum :default "ActorDestroyed"))
  (Class|VictoryCore|RemoveActorfromCustomActorList (Class|Actor|GetWorld) "ImpLystro" self))

(fn ConstructionScript
  (bind _self self)
  (|CallParentFunction)
  (bind _asshootergamemode (Utilities|Casting|CastToShooterGameMode (Game|GetGameMode)))
  (bind _returnvalue (Class|ShooterGameMode|GetIntOptionIni _asshootergamemode "ImpLystro" "MaxWildCount"))
  (Variables|Default|SetMaxWildCount (Math|Integer|SelectInt _returnvalue (Variables|Default|GetMaxWildCount) (> _returnvalue 0)))
  (bind _returnvalue_2 (Class|VictoryCore|ServerOctreeOverlapActorsClass (Class|Actor|GetWorld _self) (Transformation|GetActorLocation _self) 5e+04 "DINOPAWNS" (Variables|Default|GetMyClass) false))
  (Variables|Default|SetWildinArea _returnvalue_2))

(fn BPGetMultiUseEntries
  (params (ForPC :type Player%20Controller%20Object%20Reference) (MultiUseEntries :type Array%20of%20Multi%20Use%20Entry%20Structures))
  (if (== (Variables|/Script/Engine.Actor|GetTargetingTeam ForPC) (Variables|Default|GetTargetingTeam))
    (bind _result (CallFunction|HasXPBuff))
    (if (Math|Boolean|ANDBoolean (not _result) (not (Variables|Default|GetbIsBaby)) (Class|PrimalCharacter|BPIsConscious))
      (Utilities|Array|Add MultiUseEntries (Utilities|Struct|MakeMultiUseEntry 0 "Pet It" 367 10000 false false false false true))))
  (return MultiUseEntries))

(fn HasXPBuff
  (LocalVariables|SetRetVal false)
  (bind _array_element (Utilities|Array|ForEachLoopwithBreak (Class|PrimalCharacter|GetBuffs) :!label _label)
    (:LoopBody
      (Utilities|Casting|CastToBuff_XPLystro _array_element)
      (LocalVariables|SetRetVal true)
      (goto _label Break))
    (:Completed
      (return (LocalVariables|GetRetVal)))))

(fn BPTryMultiUse
  (params (ForPC :type Player%20Controller%20Object%20Reference) (UseIndex :type Integer))
  (bind _petanims (Variables|Default|GetPetAnims))
  (switch int UseIndex
    (:Default
      (return true))
    (:367
      (Class|PrimalBuff|StaticAddBuff "/Game/Mods/NAMC/CoreBlueprints/Buffs/Buff_XPImpLystro.Buff_XPImpLystro_C" self 0 0 false)
      (Utilities|FlowControl|Sequence
        (:then_0
          (Class|PrimalCharacter|PlayAnimEx (Utilities|Array|Get(acopy) _petanims (Math|Random|RandomIntegerinRange 0 (- (Utilities|Array|Length _petanims) 1))) 1.0 "None" true false false true false 0.0 0.0)
          (bind _asshooterplayercontroller (Utilities|Casting|CastToShooterPlayerController ForPC))
          (Class|PrimalCharacter|PlayAnimEx (Class|ShooterPlayerController|GetPlayerCharacter _asshooterplayercontroller) "/Game/PrimalEarth/Human/Male/Animations/Human-Pickup_Montage.Human-Pickup_Montage" 1.0 "None" true true false false false 0.0 0.0))
        (:then_1
          (return true))))))

(fn OnRepDinoName)
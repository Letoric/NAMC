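; Equus dino character implementing ride-to-tame: feeding the wild animal unlocks riding, and mounting swaps in buck-taming movement and stat settings.
; A server timer picks wander destinations and triggers timed bucks, while a non-dedicated timer steers toward the destination.
; Feeding from the rider's inventory during a buck adds team-locked affinity until tamed.
; Mistimed feeding, missed bucks or lingering in water force dismount, costing affinity and effectiveness and drawing aggro.
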(event Custom|ThrowPlayerOrTame
  (params (BuckAnimLength :type Float%20%28single-precision%29))
  ;[0.9061 0.4813 1] Throw Player/Tame Dino (Called from Server Timer) or on input
  (Utilities|FlowControl|Delay BuckAnimLength)
  (if (Variables|Local/DoNotEdit|GetbIsBucking)
    (if (Variables|Local/DoNotEdit|GetbDidFeed)
      ;[0.005352 0.5 0] Progress Tame
      (Utilities|FlowControl|Sequence
        (:then_0
          (Class|PrimalCharacter|PlayAnimEx (Variables|Default|GetFedDuringBuckAnim) 1.0 "None" true true false false false 0.0 0.0)
          (CallFunction|IncreaseTamingAffinity))
        (:then_1
          (if (>= (Variables|Default|GetCurrentTameAffinity) (Variables|Default|GetRequiredTameAffinity))
            (Class|PrimalCharacter|PlayAnimEx (Variables|Default|GetBabyCuddledAnimation) 1.0 "None" true true false false false 0.0 0.0)
            (Class|PrimalDinoCharacter|TameDino 0 false 0 false false false))
          ;[0 0 0] Clear Variables
          (CallFunction|ClearBucking :!label _label)))
      (else
        ;[1 0.5287 0.1006] Force dismount, fail taming
        (CallFunction|ForceDismount)
        (CallFunction|RespondtoDismount)
        (goto _label)))))

(event Custom|StartMount
  (params (TargetPlayer :type Shooter%20Character%20Object%20Reference))
  ;[0 0.03269 0.51] Start Mount and Setup Stats
  (Variables|Local/DoNotEdit|SetTamingPlayerTarget TargetPlayer)
  (Class|PrimalBuff|StaticAddBuff "/Game/PrimalEarth/CoreBlueprints/Buffs/Buff_IsTameRiding.Buff_IsTameRiding_C" TargetPlayer 0 self false)
  (BuckTaming|SetupBuckTamingStats)
  (Class|PrimalCharacter|StopAnimEx (Variables|Default|GetWakingConsumeFoodAnim) true true 0.2))

(event Custom|PathingInput
  (bind _returnvalue (Pawn|GetControlRotation :!class /Script/Engine.Pawn))
  (bind _returnvalue_2 (Transformation|GetActorForwardVector))
  (bind _returnvalue_3 (Transformation|GetActorLocation))
  (bind _myrandomdestination (Variables|Local/DoNotEdit|GetMyRandomDestination))
  (bind _returnvalue_4 (- _myrandomdestination _returnvalue_3))
  (bind _returnvalue_5 (Math|Rotator|MakeRotfromX _returnvalue_4))
  (bind _returnvalue_6 (Math|Vector|Normalize _returnvalue_4))
  (bind _yaw (Class|KismetMathLibrary|BreakRot _returnvalue_5))
  (bind _returnvalue_7 (+ _returnvalue_6 _returnvalue_2))
  (bind (_x _y) (Math|Vector|BreakVector _returnvalue_7))
  ;[1 0.08995 0.0995] Pathing Input based on random destination
  (Pawn|SetControlRotation (Pawn|GetController) (Class|KismetMathLibrary|RInterptoConstant _returnvalue (Class|KismetMathLibrary|MakeRot 0.0 _yaw 0.0) (Utilities|Time|GetWorldDeltaSeconds) (Math|Float|Clamp(Float) (* (Math|Float|Absolute(Float) (- (.Yaw (Class|KismetMathLibrary|BreakRot _returnvalue)) _yaw)) 4.0) 5e+01 3e+02)))
  (Class|PawnMovementComponent|AddInputVector (Variables|Character|GetCharacterMovement) (* (Math|Vector|MakeVector _x _y 2e+01) (* (Variables|/Script/Engine.CharacterMovementComponent|GetMaxWalkSpeed (Variables|Character|GetCharacterMovement)) (Variables|Default|GetRunningSpeedModifier) (Variables|Default|GetUntamedRunningSpeedModifier))) true)
  (Utilities|FlowControl|Sequence
    (:then_0
      (if (not (Class|PrimalCharacter|IsRunning))
        (Class|PrimalCharacter|OnStartRunning)))
    (:then_1
      (if (Variables|Default|GetbTest)
        (Rendering|Debug|DrawDebugSphere (Variables|Local/DoNotEdit|GetMyRandomDestination) 3e+02 12 "(R=1.000000,G=1.000000,B=1.000000,A=1.000000)" 0.2)))))

(event Custom|SetAllowRiding
  (params (ShouldAllow :type Boolean))
  ;[0.3424 0.6931 1] Set Allow Riding
  (Variables|Default|SetbRidingRequiresTamed (not ShouldAllow)))

(event Custom|Server_PlayStoleFoodSound
  ;[0 1 0.1993] Fed Sound
  (Utilities|FlowControl|DoOnce false :!label _label
    (:Completed
      (Utilities|FlowControl|Sequence
        (:then_0
          (Class|GameplayStatics|PlaySoundAttached (Variables|Default|GetFedDuringBuckSound) (Variables|Character|GetMesh) "MeleeSocket" "0, 0, 0" "SnapToTarget"))
        (:then_1
          (Utilities|FlowControl|Delay 3.0)
          (goto _label Reset))))))

(event Custom|Multi_UpdateRandomDestination
  (params (Destination :type Vector))
  ;[0.625 0 0.3841] Setup Pathing
  (Variables|Local/DoNotEdit|SetMyLastRandomDestination (Variables|Local/DoNotEdit|GetMyRandomDestination))
  (Variables|Local/DoNotEdit|SetMyRandomDestination Destination))

(event Custom|ThrowOrTameNoDelay
  ;[0.9061 0.4813 1] Throw Player/Tame Dino (Called from Server Timer) or on input
  (if (Variables|Local/DoNotEdit|GetbIsBucking)
    (if (Variables|Local/DoNotEdit|GetbDidFeed)
      ;[0.005352 0.5 0] Progress Tame
      (Utilities|FlowControl|Sequence
        (:then_0
          (Class|PrimalCharacter|PlayAnimEx (Variables|Default|GetFedDuringBuckAnim) 1.0 "None" true true false false false 0.0 0.0)
          (CallFunction|IncreaseTamingAffinity))
        (:then_1
          (if (>= (Variables|Default|GetCurrentTameAffinity) (Variables|Default|GetRequiredTameAffinity))
            (Class|PrimalCharacter|PlayAnimEx (Variables|Default|GetBabyCuddledAnimation) 1.0 "None" true true false false false 0.0 0.0)
            (Class|PrimalDinoCharacter|TameDino 0 false 0 false false false))
          ;[0 0 0] Clear Variables
          (CallFunction|ClearBucking :!label _label)))
      (else
        ;[1 0.5287 0.1006] Force dismount, fail taming
        (CallFunction|ForceDismount)
        (CallFunction|RespondtoDismount)
        (goto _label)))))

(event Custom|ClearBucking
  ;[0 0 0] Clear Variables
  (Variables|Local/DoNotEdit|SetbIsBucking false true)
  (Variables|Local/DoNotEdit|SetbDidFeed false)
  (Variables|Local/DoNotEdit|SetAffinityIncreaseForFoodItem 0.0))

(event Custom|Server_PlayFedSound
  ;[0 1 0.1993] Fed Sound
  (Utilities|FlowControl|DoOnce false :!label _label
    (:Completed
      (Utilities|FlowControl|Sequence
        (:then_0
          (Class|GameplayStatics|PlaySoundAttached (Variables|Default|GetFedDuringBuckSound) (Variables|Character|GetMesh) "MeleeSocket" "0, 0, 0" "SnapToTarget"))
        (:then_1
          (Utilities|FlowControl|Delay 3.0)
          (goto _label Reset))))))

(event Custom|RespondToDismount
  ;[0.9969 1 0.035] Respond to Dismount
  (Utilities|FlowControl|Delay 0.2)
  (Class|PrimalDinoCharacter|DoAttack 1 true false)
  (Class|PawnMovementComponent|AddInputVector (Variables|Character|GetCharacterMovement) "0, 0, 0" true)
  (Utilities|FlowControl|Delay 7.0)
  (BuckTaming|ResetBuckTamingStats false)
  (Class|PrimalCharacter|OnStopRunning))

(event Custom|Server_Path
  ;[0.625 0 0.3841] Setup Pathing
  (CallFunction|PathingInput))

(fn ConstructionScript
  (|CallParentFunction))

(fn BPUntamedConsumeFoodItem
  (params (foodItem :type Primal%20Item%20Object%20Reference))
  (CallFunction|SetAllowRiding true))

(fn BPTimerServer
  (bind _charactermovement (Variables|Character|GetCharacterMovement))
  (bind _movementmode (Variables|/Script/Engine.CharacterMovementComponent|GetMovementMode _charactermovement))
  (if (and (not (Class|PrimalDinoCharacter|BPIsTamed)) (Utilities|IsValid (Variables|Default|GetRider)))
    (if (not (Utilities|Enum|Equal(Enum) (Variables|/Script/Engine.CharacterMovementComponent|GetMovementMode (Variables|Character|GetCharacterMovement)) "MOVE_Walking"))
      ;[1 0.4515 0.3749] Deal with water: Dismount if we've been in too long, otherwise try to path to ground or forward
      (if (and (Class|VictoryCore|IsTimeSince (Class|Actor|GetWorld) (Variables|Local/DoNotEdit|GetLastBuckTime) (Variables|Default|GetMaxTimeTillBuck) false) (or (Utilities|Enum|Equal(Enum) _movementmode "MOVE_Swimming") (Utilities|Enum|Equal(Enum) _movementmode "MOVE_None")))
        (CallFunction|ForceDismount)
        (CallFunction|RespondtoDismount)
        (else
          ;[0.156 1 0.245] Update random move target
          (if (or (Class|VictoryCore|IsTimeSince (Class|Actor|GetWorld) (Variables|Local/DoNotEdit|GetLastRandomLocationUpdateTime) (Variables|Default|GetRandomDestinationMaxTimeToChange) true) (<= (Math|Vector|VectorLength (- (Transformation|GetActorLocation) (Variables|Local/DoNotEdit|GetMyRandomDestination))) (Variables|Default|GetRandomDestinationAcceptanceRadius))) :!label _label
            (bind _newlocationpoint (CallFunction|UpdateRandomLocation))
            (CallFunction|MultiUpdateRandomDestination _newlocationpoint)
            (Variables|Local/DoNotEdit|SetLastRandomLocationUpdateTime (Utilities|Time|GetGameTimeinSeconds)))))
      (else
        (Utilities|FlowControl|Sequence
          (:then_0
            (goto _label))
          (:then_1
            ;[0.3011 0.3467 1] Buck
            (if (Class|VictoryCore|IsTimeSince (Class|Actor|GetWorld) (Variables|Local/DoNotEdit|GetLastBuckTime) (Math|Float|SelectFloat (Variables|Default|GetMinTimeTillBuck) (Variables|Local/DoNotEdit|GetRandTimeTillBuck) (<= (Variables|Local/DoNotEdit|GetRandTimeTillBuck) 0.0)) true)
              (Variables|Local/DoNotEdit|SetbIsBucking true true)
              (Class|PrimalCharacter|PlayAnimEx (Variables|Default|GetRider) (Variables|Default|GetHumanBuckAnim) 1.0 "None" true true false false false 0.0 0.0)
              (bind _returnvalue (Class|PrimalCharacter|PlayAnimEx (Variables|Default|GetBuckAnim) 1.0 "None" true true false false false 0.0 0.0))
              (CallFunction|ThrowPlayerorTame _returnvalue)
              (Variables|Local/DoNotEdit|SetLastBuckTime (Utilities|Time|GetGameTimeinSeconds))
              (Variables|Local/DoNotEdit|SetRandTimeTillBuck (Math|Random|RandomFloatinRange (Variables|Default|GetMinTimeTillBuck) (Variables|Default|GetMaxTimeTillBuck))))))))
    (else
      (BuckTaming|ResetBuckTamingStats false))))

(fn BPNotifySetRider
  (params (RiderSetting :type Shooter%20Character%20Object%20Reference))
  (if (not (Class|PrimalDinoCharacter|BPIsTamed))
    (if (not (== RiderSetting 0))
      (CallFunction|StartMount RiderSetting))))

(fn ConsumeValidFood
  (LocalVariables|SetRetDidConsumeFood false)
  (LocalVariables|SetRetEffectivenessMultiplier 1.0)
  (Utilities|FlowControl|Sequence
    (:then_0
      ;[0.086 0.1926 1] Get real affinity increase
      (bind _returnvalue (Class|PrimalDinoCharacter|GetAffinityIncreaseforFoodItem (Utilities|Array|Get(acopy) (Variables|/Script/ShooterGame.PrimalInventoryComponent|GetItemSlots (Variables|/Script/ShooterGame.PrimalCharacter|GetMyInventoryComponent (Variables|Default|GetRider))) 9)))
      (if (> _returnvalue 0.0)
        (LocalVariables|SetRetDidConsumeFood true)
        (LocalVariables|SetRetEffectivenessMultiplier _returnvalue)
        (Class|PrimalDinoCharacter|BPConsumeInventoryFoodItem (Utilities|Array|Get(acopy) (Variables|/Script/ShooterGame.PrimalInventoryComponent|GetItemSlots (Variables|/Script/ShooterGame.PrimalCharacter|GetMyInventoryComponent (Variables|Default|GetRider))) 9) false)))
    (:then_1
      ;[0.1812 0.885 1] Return and respond to food consumption
      (if (LocalVariables|GetRetDidConsumeFood)
        (if (Variables|Local/DoNotEdit|GetbIsBucking)
          (CallFunction|ServerPlayFedSound)
          (else
            (CallFunction|ServerPlayStoleFoodSound))))
      (return (LocalVariables|GetRetDidConsumeFood) (LocalVariables|GetRetEffectivenessMultiplier)))))

(fn ForceDismount
  (Class|PrimalDinoCharacter|ForceClearRider)
  (bind _asdino_aicontroller_bp_c (Utilities|Casting|CastToDino_AIController_BP (Pawn|GetController))
    (:then
      (Class|PrimalDinoAIController|AddtoAggro _asdino_aicontroller_bp_c (Variables|Local/DoNotEdit|GetTamingPlayerTarget) 1.0 false true true false))
    (:CastFailed
      _))
  (CallFunction|ClearBucking)
  (if (Networking|IsServer)
    (Variables|Default|SetCurrentTameAffinity (Math|Float|Max(Float) (- (Variables|Default|GetCurrentTameAffinity) (Math|Float|Max(Float) (* (Variables|Default|GetCurrentTameAffinity) (Variables|Default|GetDismountAffinityLostPercentage) 0.01) 1e+01)) 0.0) true)
    (Variables|Default|SetTameIneffectivenessModifier (+ (Variables|Default|GetTameIneffectivenessModifier) (Math|Float|Max(Float) (* (Variables|Default|GetTameIneffectivenessModifier) (Variables|Default|GetDismountTameIneffectivenessMultiplier)) (Variables|Default|GetDismountTameIneffectivenessMinimum))) true))
  (return))

(fn BPPreventInputType
  (params (inputType :type EPrimalCharacterInputType%20Enum :default "PrimaryFire"))
  (return (and (not (Class|PrimalDinoCharacter|BPIsTamed)) (Variables|Default|GetbHasRider))))

(fn BPSetupTamed
  (params (bWasJustTamed :type Boolean))
  (bind _rider (Variables|Default|GetRider))
  (Variables|/Script/Engine.CharacterMovementComponent|SetMass (Variables|Character|GetCharacterMovement) 2e+02)
  (BuckTaming|ResetBuckTamingStats bWasJustTamed)
  (Class|PrimalCharacter|OnStopRunning)
  (Variables|Default|SetbUseBPTimerNonDedicated false)
  (Utilities|IsValid _rider
    (:Is%20Valid
      (Class|PrimalCharacter|DeactivateBuffs _rider "/Game/PrimalEarth/CoreBlueprints/Buffs/Buff_IsTameRiding.Buff_IsTameRiding_C" 0 false))))

(fn ResetBuckTamingStats
  (params (ForceReset :type Boolean))
  (bind _mycharacterstatuscomponent (Variables|Default|GetMyCharacterStatusComponent))
  (Utilities|FlowControl|Sequence
    (:then_0
      (if (or ForceReset (or (Class|PrimalDinoCharacter|BPIsTamed) (not (Variables|Default|GetbHasRider))))
        (Utilities|FlowControl|Sequence
          (:then_0
            (bind _returnvalue (Class|VictoryCore|GetDefaultObject self))
            (bind _asprimaldinocharacter (Utilities|Casting|CastToPrimalDinoCharacter _returnvalue))
            (Utilities|FlowControl|Sequence
              (:then_0
                (Variables|Default|SetWildRunningRotationRateModifier (Variables|/Script/ShooterGame.PrimalDinoCharacter|GetWildRunningRotationRateModifier _asprimaldinocharacter)))
              (:then_1
                (Variables|/Script/Engine.CharacterMovementComponent|SetRotationAcceleration (Variables|Character|GetCharacterMovement) (Variables|/Script/Engine.CharacterMovementComponent|GetRotationAcceleration (Variables|/Script/Engine.Character|GetCharacterMovement _asprimaldinocharacter))))))
          (:then_1
            (bind _returnvalue_2 (Class|VictoryCore|GetDefaultObject _mycharacterstatuscomponent))
            (bind _asprimalcharacterstatuscomponent (Utilities|Casting|CastToPrimalCharacterStatusComponent _returnvalue_2))
            (Variables|/Script/ShooterGame.PrimalCharacterStatusComponent|SetFoodConsumptionMultiplier _mycharacterstatuscomponent (Variables|/Script/ShooterGame.PrimalCharacterStatusComponent|GetFoodConsumptionMultiplier _asprimalcharacterstatuscomponent))
            (Variables|/Script/ShooterGame.PrimalCharacterStatusComponent|SetRunningStaminaConsumptionRate _mycharacterstatuscomponent (Variables|/Script/ShooterGame.PrimalCharacterStatusComponent|GetRunningStaminaConsumptionRate _asprimalcharacterstatuscomponent)))
          (:then_2
            (Variables|Default|SetbUseBPTimerServer false))
          (:then_3
            (if (Math|Float|NearlyEqual(Float) (Variables|Default|GetCurrentTameAffinity) 0.0 0.001)
              (CallFunction|SetAllowRiding false))))))
    (:then_1
      (return))))

(fn BPDoAttack
  (params (AttackIndex :type Integer))
  (bind _rider (Variables|Default|GetRider))
  (switch int AttackIndex
    (:3
      (if (Variables|Local/DoNotEdit|GetbIsBucking)
        (if (not (Variables|Local/DoNotEdit|GetbDidFeed))
          (bind (_didconsumefood _effectivenessmultiplier) (CallFunction|ConsumeValidFood))
          (Variables|Local/DoNotEdit|SetbDidFeed _didconsumefood)
          (Variables|Local/DoNotEdit|SetAffinityIncreaseForFoodItem _effectivenessmultiplier)
          (Class|PrimalCharacter|StopAnimEx _rider (Variables|Default|GetHumanBuckAnim) true true 0.2)
          (Class|PrimalCharacter|PlayAnimEx _rider (Variables|Default|GetHumanFedAnim) 1.0 "None" true true false false false 0.0 0.0)
          (Class|PrimalCharacter|StopAnimEx (Variables|Default|GetBuckAnim) true true 0.2)
          (CallFunction|ThroworTameNoDelay))
        (else
          (CallFunction|ConsumeValidFood)
          (CallFunction|ForceDismount)
          (CallFunction|RespondtoDismount))))))

(fn IncreaseTamingAffinity
  (bind _rider (Variables|Default|GetRider))
  (bind _affinityperbuckmultiplier (Variables|Default|GetAffinityPerBuckMultiplier))
  (bind _affinityincreaseforfooditem (Variables|Local/DoNotEdit|GetAffinityIncreaseForFoodItem))
  (bind _returnvalue (* _affinityperbuckmultiplier _affinityincreaseforfooditem))
  (if (== 0 (Variables|Default|GetTamingTeamID))
    (bind _asshootercharacter (Utilities|Casting|CastToShooterCharacter _rider)
      (:then
        (Variables|Default|SetTamingTeamID (Variables|/Script/Engine.Actor|GetTargetingTeam _asshootercharacter) false)
        (Variables|Default|SetCurrentTameAffinity (+ (Variables|Default|GetCurrentTameAffinity) _returnvalue) false)
        (Class|PrimalDinoCharacter|NetUpdateDinoNameStrings (Variables|/Script/ShooterGame.PrimalCharacter|GetTribeName _asshootercharacter))
        (Variables|Local/DoNotEdit|SetLastTimeRecievedAffinity (Utilities|Time|GetGameTimeinSeconds)))
      (:CastFailed
        _))
    (return)
    (else
      (bind _asshootercharacter_2 (Utilities|Casting|CastToShooterCharacter _rider)
        (:then
          (if (== (Variables|/Script/Engine.Actor|GetTargetingTeam _asshootercharacter_2) (Variables|Default|GetTamingTeamID))
            (Variables|Default|SetCurrentTameAffinity (+ (Variables|Default|GetCurrentTameAffinity) _returnvalue) false)
            (Variables|Local/DoNotEdit|SetLastTimeRecievedAffinity (Utilities|Time|GetGameTimeinSeconds))
            (return)))
        (:CastFailed
          (return))))))

(fn UpdateRandomLocation
  (LocalVariables|SetRetFoundPoint false)
  (LocalVariables|SetTempLocation "0, 0, 0")
  (if (Networking|IsServer)
    (Utilities|FlowControl|Sequence
      (:then_0
        ;[0.242 0.8946 1] Give multiple attempts to find a good point
        (Utilities|FlowControl|ForLoopwithBreak 0 2 :!label _label
          (:LoopBody
            (if (== (LocalVariables|GetTempLocation) "0, 0, 0")
              ;[0.2575 0.4499 1] Get controller and random point
              (bind _returnvalue (Class|VictoryCore|GetClassDefaultObject "/Game/Mods/NAMC/Dinos/Equus/Equus_AI_Blueprint.Equus_AI_Blueprint_C"))
              (bind _asprimaldinoaicontroller (Utilities|Casting|CastToPrimalDinoAIController _returnvalue))
              (bind _returnvalue_2 (Class|PrimalDinoAIController|StaticGetRandomWanderDestination _asprimaldinoaicontroller self _asprimaldinoaicontroller "0, 0, 0" (Math|Float|SelectFloat 3.0 1.0 (Utilities|Enum|Equal(Enum) (Variables|/Script/Engine.CharacterMovementComponent|GetMovementMode (Variables|Character|GetCharacterMovement)) "MOVE_Swimming")) true false "0, 0, 0" (Variables|Default|GetRandomDestGroundCheckSpread)))
              (LocalVariables|SetTempLocation _returnvalue_2)
              (else
                (goto _label Break))))
          (:Completed
            ;[1 0.3894 0.7111] Deal with bad locations, worst  case run in circles
            (if (== (LocalVariables|GetTempLocation) "0, 0, 0")
              (if (== (Variables|Local/DoNotEdit|GetMyLastRandomDestination) "0, 0, 0")
                (LocalVariables|SetTempLocation (+ (Transformation|GetActorLocation) (* (Transformation|GetActorForwardVector) (Math|Float|SelectFloat 1e+03 -1e+03 (Utilities|Enum|Equal(Enum) (Variables|/Script/Engine.CharacterMovementComponent|GetMovementMode (Variables|Character|GetCharacterMovement)) "MOVE_Swimming")))))
                (else
                  (LocalVariables|SetTempLocation (Variables|Local/DoNotEdit|GetMyLastRandomDestination))))
              (else
                (LocalVariables|SetRetFoundPoint true))))))
      (:then_1
        (return (LocalVariables|GetRetFoundPoint) (LocalVariables|GetTempLocation))))
    (else
      (return (LocalVariables|GetRetFoundPoint) (LocalVariables|GetTempLocation)))))

(fn BPTimerNonDedicated
  (if (Math|Boolean|ANDBoolean (not (Class|PrimalDinoCharacter|BPIsTamed)) (Utilities|IsValid (Variables|Default|GetRider)) (not (Variables|Local/DoNotEdit|GetbIsBucking)))
    (Utilities|FlowControl|Sequence
      (:then_0
        (CallFunction|ServerPath))
      (:then_1
        (CallFunction|PathingInput)))))

(fn BPGetMultiUseEntries
  (params (ForPC :type Player%20Controller%20Object%20Reference) (MultiUseEntries :type Array%20of%20Multi%20Use%20Entry%20Structures))
  (if (not (Class|PrimalDinoCharacter|BPIsTamed))
    ;[1 0.4943 0.7011] Prevent riding if they aren't on the right team or are in water
    (for (_array_element _array_index) MultiUseEntries
      (if (and (or (!= (Variables|/Script/Engine.Actor|GetTargetingTeam ForPC) (Variables|Default|GetTamingTeamID)) (Utilities|Enum|Equal(Enum) (Variables|/Script/Engine.CharacterMovementComponent|GetMovementMode (Variables|Character|GetCharacterMovement)) "MOVE_Swimming")) (== (.UseIndex (Utilities|Struct|BreakMultiUseEntry _array_element)) 100))
        (Utilities|Array|SetArrayElem MultiUseEntries _array_index (Utilities|Struct|MakeMultiUseEntry (.ForComponent (Utilities|Struct|BreakMultiUseEntry _array_element)) (.UseString (Utilities|Struct|BreakMultiUseEntry _array_element)) 0 (.Priority (Utilities|Struct|BreakMultiUseEntry _array_element)) (.bHideFromUI (Utilities|Struct|BreakMultiUseEntry _array_element)) (or true (.bDisableUse (Utilities|Struct|BreakMultiUseEntry _array_element))) (.bHideActivationKey (Utilities|Struct|BreakMultiUseEntry _array_element)) (.bRepeatMultiUse (Utilities|Struct|BreakMultiUseEntry _array_element)) (.bDisplayOnInventoryUI (Utilities|Struct|BreakMultiUseEntry _array_element)) (.bDisplayOnInventoryUISecondary (Utilities|Struct|BreakMultiUseEntry _array_element)) (.bHarvestable (Utilities|Struct|BreakMultiUseEntry _array_element)) (.bIsSecondaryUse (Utilities|Struct|BreakMultiUseEntry _array_element)) (.bPersistWheelOnActivation (Utilities|Struct|BreakMultiUseEntry _array_element)) (.bOverrideUseTextColor (Utilities|Struct|BreakMultiUseEntry _array_element)) false false false false (.WheelCategory (Utilities|Struct|BreakMultiUseEntry _array_element)) (.DisableUseColor (Utilities|Struct|BreakMultiUseEntry _array_element)) (.UseTextColor (Utilities|Struct|BreakMultiUseEntry _array_element)) (.EntryActivationTimer (Utilities|Struct|BreakMultiUseEntry _array_element)) (.DefaultEntryActivationTimer (Utilities|Struct|BreakMultiUseEntry _array_element)) (.ActivationSound (Utilities|Struct|BreakMultiUseEntry _array_element)))))))
  (return MultiUseEntries))

(fn BPTryMultiUse
  (params (ForPC :type Player%20Controller%20Object%20Reference) (UseIndex :type Integer))
  (return true))

(fn SetupBuckTamingStats
  (bind _mycharacterstatuscomponent (Variables|Default|GetMyCharacterStatusComponent))
  (Variables|Default|SetWildRunningRotationRateModifier (Variables|BuckTaming|GetBuckTamingRunningRotationRateModifier))
  (Variables|/Script/Engine.CharacterMovementComponent|SetRotationAcceleration (Variables|Character|GetCharacterMovement) (Variables|BuckTaming|GetBuckTamingRotationAcceleration))
  (Variables|/Script/ShooterGame.PrimalCharacterStatusComponent|SetRunningStaminaConsumptionRate _mycharacterstatuscomponent 0.001)
  (Variables|/Script/ShooterGame.PrimalCharacterStatusComponent|SetFoodConsumptionMultiplier _mycharacterstatuscomponent (Variables|BuckTaming|GetBuckTamingFoodConsumptionMultiplier))
  (Variables|Default|SetbUseBPTimerServer true)
  (return))

(fn BPModifyHarvestDamage
  (params (harvestComponent :type Primal%20Harvesting%20Component%20Object%20Reference) (inDamage :type Float%20%28single-precision%29))
  (bind _returnvalue (Utilities|GetClass harvestComponent))
  (bind _currentattackindex (Variables|Default|GetCurrentAttackIndex))
  (bind _returnvalue_2 (Math|Conversions|ToInteger(Byte) _currentattackindex))
  (bind _returnvalue_3 (Utilities|ClassIsChildOf _returnvalue "/Game/PrimalEarth/CoreBlueprints/HarvestComponents/UseHarvestComponent_Base.UseHarvestComponent_Base_C"))
  (return (Math|Float|SelectFloat 0.0 inDamage (or (and (not _returnvalue_3) (== _returnvalue_2 0)) (and _returnvalue_3 (== _returnvalue_2 1))))))
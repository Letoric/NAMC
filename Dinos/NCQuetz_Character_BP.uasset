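; Quetzal dino character (NCQuetz) that applies server INI tuning for grab weight, platform structures, item weight, fly speed and wild population.
; On BeginPlay it records wild stat points, scales untamed fly speed by level tier, and starts a timer that culls stasised wild Quetzals found nearby at construction.
; On taming it reapplies speed, sets stats above MaxAllowedLevels or below recorded values to that cap, then recomputes base level.
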(event `self.ReceiveEndPlay`
  (params (EndPlayReason :type "EngineTypes.EEndPlayReason Enum" :default "ActorDestroyed"))
  (`VictoryCore.RemoveActorFromCustomActorList` (`self.K2_GetWorld`) "NCQuetz" self))

(event `Purge`
  (bind _wildinarea (`self.WildinArea`))
  (bind _item (`KismetArrayLibrary.Array_Get` _wildinarea))
  (if (> (`KismetArrayLibrary.Array_Length` _wildinarea) (`KismetMathLibrary.Min` (/ (`self.MaxWildCount`) 5) 1))
    (bind _asncquetz_character_bp_c (cast `/Dinos/NCQuetz_Character_BP` _item)
      (:`then`
        (if (and (not (`self.BPIsTamed` _asncquetz_character_bp_c)) (`Actor.bStasised` _asncquetz_character_bp_c))
          (`/Engine/EditorBlueprintResources/StandardMacros.IsValid` _item
            (:`Is Valid`
              (`VictoryCore.RemoveActorFromCustomActorList` (`self.K2_GetWorld`) "NCQuetz" _asncquetz_character_bp_c)
              (`self.K2_DestroyActor` _item))
            (:`Is Not Valid`
              (`VictoryCore.RemoveActorFromCustomActorList` (`self.K2_GetWorld`) "NCQuetz" _asncquetz_character_bp_c)))))
      (:`CastFailed`
        _))
    (`KismetArrayLibrary.Array_Remove` _wildinarea)
    (`KismetSystemLibrary.K2_SetTimer` null "Purge" 2.0)
    (else
      (`KismetSystemLibrary.K2_ClearTimer` null "Purge"))))

(event `self.ReceiveBeginPlay`
  (bind _maxflyspeed_30 (`self.MaxFlySpeed_30`))
  (bind _maxflyspeed (`self.MaxFlySpeed`))
  (bind _shootergamemoderef (`self.ShooterGameModeRef`))
  (bind _returnvalue (- _maxflyspeed_30 _maxflyspeed))
  (bind _itemclassweightmultipliers (`PrimalInventoryComponent.ItemClassWeightMultipliers` (`self.MyInventoryComponent`)))
  (bind _basecharacterlevel (`PrimalCharacterStatusComponent.BaseCharacterLevel` (`self.DinoCharacterStatus_BP_NCQuetz_C1`)))
  (bind _returnvalue_2 (`KismetMathLibrary.FFloor` (`ShooterGameMode.DifficultyValue` (`self.ShooterGameModeRef`))))
  (`KismetSystemLibrary.Delay` 0.2)
  (`/Engine/EditorBlueprintResources/ActorMacros.SwitchNetAuthority`
    (:`DedicatedServer`
      (bind _asshootergamemode (cast `ShooterGameMode` (`GameplayStatics.GetGameMode`) :!label _label))
      (set `self.ShooterGameModeRef` _asshootergamemode)
      (`|ExecutionSequence`
        (:`then_0`
          ;[1 1 1] Set Variables from INI or Set pre-defined value
          (bind _returnvalue_3 (`ShooterGameMode.GetFloatOptionIni` _shootergamemoderef "NCQuetzal" "GrabWeightMax"))
          (set `self.GrabWeightThreshold` (`KismetMathLibrary.SelectFloat` (`self.GrabWeightThreshold`) _returnvalue_3 (<= _returnvalue_3 0.0)))
          (bind _returnvalue_4 (`ShooterGameMode.GetIntOptionIni` _shootergamemoderef "NCQuetzal" "MaxPlatformStructures"))
          (set `self.MaxSaddleStructuresNum` (`KismetMathLibrary.SelectInt` (`self.MaxSaddleStructuresNum`) _returnvalue_4 (<= _returnvalue_4 0)))
          (bind _returnvalue_5 (`ShooterGameMode.GetFloatOptionIni` _shootergamemoderef "NCQuetzal" "ItemWeightMulti"))
          (set `self.ItemWeightMulti` (`KismetMathLibrary.SelectFloat` (`self.ItemWeightMulti`) _returnvalue_5 (<= _returnvalue_5 0.0)))
          (bind _returnvalue_6 (`ShooterGameMode.GetFloatOptionIni` _shootergamemoderef "NCQuetzal" "MaxFlySpeed"))
          (set `self.MaxFlySpeed_30` (`KismetMathLibrary.SelectFloat` (`self.MaxFlySpeed`) _returnvalue_6 (<= _returnvalue_6 0.0)) false)
          (bind _returnvalue_7 (`ShooterGameMode.GetIntOptionIni` _shootergamemoderef "NCQuetzal" "MaxWildCount"))
          (set `self.MaxWildCount` (`KismetMathLibrary.SelectInt` _returnvalue_7 (`self.MaxWildCount`) (> _returnvalue_7 0))))
        (:`then_1`
          (`KismetSystemLibrary.K2_SetTimer` null "Purge" 2.0))
        (:`then_2`
          (`|ExecutionSequence`
            (:`then_0`
              ;[1 1 1] Update Item Weight Modifier
              (for (_array_element _array_index) _itemclassweightmultipliers
                (bind _asprimalitemresourcegeneric_c (castclass `/Game/PrimalEarth/CoreBlueprints/Resources/PrimalItemResourceGeneric` (`.ItemClass` (break `ItemMultiplier` _array_element))))
                (`KismetArrayLibrary.Array_Set` _itemclassweightmultipliers _array_index (make `ItemMultiplier` _asprimalitemresourcegeneric_c (`self.ItemWeightMulti`)))))
            (:`then_1`
              (bind _asprimaldinocharacter (cast `PrimalDinoCharacter` self))
              (bind _returnvalue_8 (`self.GetCharacterStatusComponent` _asprimaldinocharacter))
              (set `self.InitHealth` (`PrimalCharacterStatusComponent.GetLevelUpPoints` _returnvalue_8 "Health" false))
              (set `self.InitStamina` (`PrimalCharacterStatusComponent.GetLevelUpPoints` _returnvalue_8 "Stamina" false))
              (set `self.InitOxygen` (`PrimalCharacterStatusComponent.GetLevelUpPoints` _returnvalue_8 "Oxygen" false))
              (set `self.InitFood` (`PrimalCharacterStatusComponent.GetLevelUpPoints` _returnvalue_8 "Food" false))
              (set `self.InitWeight` (`PrimalCharacterStatusComponent.GetLevelUpPoints` _returnvalue_8 "Weight" false))
              (set `self.InitDamage` (`PrimalCharacterStatusComponent.GetLevelUpPoints` _returnvalue_8 "MeleeDamageMultiplier" false))
              (set `self.InitSpeed` (`PrimalCharacterStatusComponent.GetLevelUpPoints` _returnvalue_8 "SpeedMultiplier" false))
              (set `self.InitCraftSpeed` (`PrimalCharacterStatusComponent.GetLevelUpPoints` _returnvalue_8 "CraftingSpeedMultiplier" false)))
            (:`then_2`
              ;[1 1 1] Update Max Fly Speed
              (if (>= _maxflyspeed_30 _maxflyspeed) :!label _label_2
                (if (`self.BPIsTamed`)
                  (set `CharacterMovementComponent.MaxFlySpeed` _maxflyspeed_30 (`self.CharacterMovement`))
                  (else
                    (set `self.MaxFlySpeed_21` (+ (`self.MaxFlySpeed`) (/ _returnvalue 2.0)))
                    (set `self.MaxFlySpeed_11` (+ (`self.MaxFlySpeed`) (/ _returnvalue 3.0)))
                    (set `self.MaxFlySpeed_1` (+ (`self.MaxFlySpeed`) (/ _returnvalue 4.0)))
                    (if (>= _basecharacterlevel (* _returnvalue_2 30))
                      (set `CharacterMovementComponent.MaxFlySpeed` (`self.MaxFlySpeed_30`) (`self.CharacterMovement`))
                      (elif (>= _basecharacterlevel (* _returnvalue_2 21))
                        (set `CharacterMovementComponent.MaxFlySpeed` (`self.MaxFlySpeed_21`) (`self.CharacterMovement`))
                        (elif (>= _basecharacterlevel (* _returnvalue_2 11))
                          (set `CharacterMovementComponent.MaxFlySpeed` (`self.MaxFlySpeed_11`) (`self.CharacterMovement`))
                          (elif (>= _basecharacterlevel (* _returnvalue_2 1))
                            (set `CharacterMovementComponent.MaxFlySpeed` (`self.MaxFlySpeed_1`) (`self.CharacterMovement`))))))))))
            (:`then_3`
              ;[1 1 1] Print Dino Info
              (bind _asprimaldinocharacter_2 (cast `PrimalDinoCharacter` self))
              (bind _returnvalue_9 (`self.GetCharacterStatusComponent` _asprimaldinocharacter_2))
              (bind (_returnvalue_x _returnvalue_y _returnvalue_z) (`KismetMathLibrary.BreakVector` (`self.K2_GetActorLocation` _asprimaldinocharacter_2)))
              (`self.Debug` (`KismetTextLibrary.Conv_TextToString` (`|FormatText` "{1},{2},{3},{4},{5},{6}" (`KismetTextLibrary.Conv_StringToText` (`KismetStringLibrary.Conv_NameToString` (`PrimalDinoCharacter.DinoNameTag` _asprimaldinocharacter_2))) (`KismetTextLibrary.Conv_StringToText` (`KismetStringLibrary.Conv_IntToString` (`PrimalCharacterStatusComponent.BaseCharacterLevel` _returnvalue_9))) (`KismetTextLibrary.Conv_StringToText` (`KismetStringLibrary.Conv_IntToString` (`KismetMathLibrary.FFloor` (`CharacterMovementComponent.MaxFlySpeed` (`self.CharacterMovement`))))) (`KismetTextLibrary.Conv_StringToText` (`KismetStringLibrary.Conv_IntToString` (`KismetMathLibrary.Round` _returnvalue_x))) (`KismetTextLibrary.Conv_StringToText` (`KismetStringLibrary.Conv_IntToString` (`KismetMathLibrary.Round` _returnvalue_y))) (`KismetTextLibrary.Conv_StringToText` (`KismetStringLibrary.Conv_IntToString` (`KismetMathLibrary.Round` _returnvalue_z)))))))
            (:`then_4`
              ;[1 1 1] Replicate
              (`KismetSystemLibrary.Delay` 0.7 :!label _label_3)
              (`self.ForceNetUpdate` false))))))
    (:`PlayerServer`
      (goto _label))
    (:`Client`
      (`KismetSystemLibrary.Delay` 1.0)
      (goto _label_2))))

(event `self.BPSetupTamed`
  (params (bWasJustTamed :type Boolean))
  (bind _maxallowedlevels (`self.MaxAllowedLevels`))
  (bind _maxallowedlevels_2 (`self.MaxAllowedLevels`))
  (bind _maxallowedlevels_3 (`self.MaxAllowedLevels`))
  (bind _maxallowedlevels_4 (`self.MaxAllowedLevels`))
  (bind _maxallowedlevels_5 (`self.MaxAllowedLevels`))
  (bind _maxallowedlevels_6 (`self.MaxAllowedLevels`))
  (bind _maxallowedlevels_7 (`self.MaxAllowedLevels`))
  (bind _maxallowedlevels_8 (`self.MaxAllowedLevels`))
  (`KismetSystemLibrary.Delay` 0.2)
  (if bWasJustTamed
    (`/Engine/EditorBlueprintResources/ActorMacros.SwitchNetAuthority`
      (:`DedicatedServer`
        (`|ExecutionSequence` :!label _label_4
          (:`then_0`
            (goto _label_2))
          (:`then_1`
            (goto _label_3))
          (:`then_2`
            _)))
      (:`PlayerServer`
        (goto _label_4))
      (:`Client`
        (`KismetSystemLibrary.Delay` 1.0)
        (`|ExecutionSequence`
          (:`then_0`
            (goto _label_2))
          (:`then_1`
            _))))
    (bind _asprimaldinocharacter (cast `PrimalDinoCharacter` self))
    (bind _returnvalue (`self.GetCharacterStatusComponent` _asprimaldinocharacter))
    (`|ExecutionSequence`
      (:`then_0`
        (`self.Debug` (`KismetStringLibrary.Concat_StrStr` "Health " (`KismetStringLibrary.Conv_IntToString` (`self.InitHealth`))) false false true 30.0)
        (`self.Debug` (`KismetStringLibrary.Concat_StrStr` "Stamina " (`KismetStringLibrary.Conv_IntToString` (`self.InitStamina`))) false false true 30.0)
        (`self.Debug` (`KismetStringLibrary.Concat_StrStr` "Oxygen " (`KismetStringLibrary.Conv_IntToString` (`self.InitOxygen`))) false false true 30.0)
        (`self.Debug` (`KismetStringLibrary.Concat_StrStr` "Food " (`KismetStringLibrary.Conv_IntToString` (`self.InitFood`))) false false true 30.0)
        (`self.Debug` (`KismetStringLibrary.Concat_StrStr` "Weight " (`KismetStringLibrary.Conv_IntToString` (`self.InitWeight`))) false false true 30.0)
        (`self.Debug` (`KismetStringLibrary.Concat_StrStr` "Melee Damage " (`KismetStringLibrary.Conv_IntToString` (`self.InitDamage`))) false false true 30.0)
        (`self.Debug` (`KismetStringLibrary.Concat_StrStr` "Speed " (`KismetStringLibrary.Conv_IntToString` (`self.InitSpeed`))) false false true 30.0)
        (`self.Debug` (`KismetStringLibrary.Concat_StrStr` "Crafting Speed " (`KismetStringLibrary.Conv_IntToString` (`self.InitCraftSpeed`))) false false true 30.0))
      (:`then_1`
        (`KismetSystemLibrary.Delay` 0.2)
        (bind _returnvalue_2 (`PrimalCharacterStatusComponent.GetLevelUpPoints` _returnvalue "Health" false))
        (if (or (> _returnvalue_2 _maxallowedlevels) (< _returnvalue_2 (`self.InitHealth`)))
          (`PrimalCharacterStatusComponent.SetLevelUpPoints` _returnvalue "Health" false _maxallowedlevels))
        (bind _returnvalue_3 (`PrimalCharacterStatusComponent.GetLevelUpPoints` _returnvalue "Stamina" false))
        (if (or (> _returnvalue_3 _maxallowedlevels_2) (< _returnvalue_3 (`self.InitStamina`)))
          (`PrimalCharacterStatusComponent.SetLevelUpPoints` _returnvalue "Stamina" false _maxallowedlevels_2))
        (bind _returnvalue_4 (`PrimalCharacterStatusComponent.GetLevelUpPoints` _returnvalue "Oxygen" false))
        (if (or (> _returnvalue_4 _maxallowedlevels_3) (< _returnvalue_4 (`self.InitOxygen`)))
          (`PrimalCharacterStatusComponent.SetLevelUpPoints` _returnvalue "Oxygen" false _maxallowedlevels_3))
        (bind _returnvalue_5 (`PrimalCharacterStatusComponent.GetLevelUpPoints` _returnvalue "Food" false))
        (if (or (> _returnvalue_5 _maxallowedlevels_4) (< _returnvalue_5 (`self.InitFood`)))
          (`PrimalCharacterStatusComponent.SetLevelUpPoints` _returnvalue "Food" false _maxallowedlevels_4))
        (bind _returnvalue_6 (`PrimalCharacterStatusComponent.GetLevelUpPoints` _returnvalue "Weight" false))
        (if (or (> _returnvalue_6 _maxallowedlevels_5) (< _returnvalue_6 (`self.InitWeight`)))
          (`PrimalCharacterStatusComponent.SetLevelUpPoints` _returnvalue "Weight" false _maxallowedlevels_5))
        (bind _returnvalue_7 (`PrimalCharacterStatusComponent.GetLevelUpPoints` _returnvalue "MeleeDamageMultiplier" false))
        (if (or (> _returnvalue_7 _maxallowedlevels_6) (< _returnvalue_7 (`self.InitDamage`)))
          (`PrimalCharacterStatusComponent.SetLevelUpPoints` _returnvalue "MeleeDamageMultiplier" false _maxallowedlevels_6))
        (bind _returnvalue_8 (`PrimalCharacterStatusComponent.GetLevelUpPoints` _returnvalue "SpeedMultiplier" false))
        (if (or (> _returnvalue_8 _maxallowedlevels_7) (< _returnvalue_8 (`self.InitSpeed`)))
          (`PrimalCharacterStatusComponent.SetLevelUpPoints` _returnvalue "SpeedMultiplier" false _maxallowedlevels_7))
        (bind _returnvalue_9 (`PrimalCharacterStatusComponent.GetLevelUpPoints` _returnvalue "CraftingSpeedMultiplier" false))
        (if (or (> _returnvalue_9 _maxallowedlevels_8) (and (< _returnvalue_9 (`self.InitCraftSpeed`)) (> _returnvalue_9 0)))
          (`PrimalCharacterStatusComponent.SetLevelUpPoints` _returnvalue "CraftingSpeedMultiplier" false _maxallowedlevels_8))
        (`PrimalCharacterStatusComponent.SetBaseLevelNoStatChange` _returnvalue (+ (+ (+ (+ (+ (+ (+ (+ _returnvalue_2 _returnvalue_3) _returnvalue_4) _returnvalue_5) _returnvalue_6) _returnvalue_7) _returnvalue_8) _returnvalue_9) 1))
        (`PrimalCharacterStatusComponent.RescaleAllStats` _returnvalue)
        (`PrimalCharacterStatusComponent.ServerSyncReplicatedValues` _returnvalue)
        (`self.Debug` (`KismetStringLibrary.Concat_StrStr` "Health " (`KismetStringLibrary.Conv_IntToString` (`PrimalCharacterStatusComponent.GetLevelUpPoints` _returnvalue "Health" false))) false false true 30.0)
        (`self.Debug` (`KismetStringLibrary.Concat_StrStr` "Stamina " (`KismetStringLibrary.Conv_IntToString` (`PrimalCharacterStatusComponent.GetLevelUpPoints` _returnvalue "Stamina" false))) false false true 30.0)
        (`self.Debug` (`KismetStringLibrary.Concat_StrStr` "Oxygen " (`KismetStringLibrary.Conv_IntToString` (`PrimalCharacterStatusComponent.GetLevelUpPoints` _returnvalue "Oxygen" false))) false false true 30.0)
        (`self.Debug` (`KismetStringLibrary.Concat_StrStr` "Food " (`KismetStringLibrary.Conv_IntToString` (`PrimalCharacterStatusComponent.GetLevelUpPoints` _returnvalue "Food" false))) false false true 30.0)
        (`self.Debug` (`KismetStringLibrary.Concat_StrStr` "Weight " (`KismetStringLibrary.Conv_IntToString` (`PrimalCharacterStatusComponent.GetLevelUpPoints` _returnvalue "Weight" false))) false false true 30.0)
        (`self.Debug` (`KismetStringLibrary.Concat_StrStr` "Melee Damage " (`KismetStringLibrary.Conv_IntToString` (`PrimalCharacterStatusComponent.GetLevelUpPoints` _returnvalue "MeleeDamageMultiplier" false))) false false true 30.0)
        (`self.Debug` (`KismetStringLibrary.Concat_StrStr` "Speed " (`KismetStringLibrary.Conv_IntToString` (`PrimalCharacterStatusComponent.GetLevelUpPoints` _returnvalue "SpeedMultiplier" false))) false false true 30.0)
        (`self.Debug` (`KismetStringLibrary.Concat_StrStr` "Crafting Speed " (`KismetStringLibrary.Conv_IntToString` (`PrimalCharacterStatusComponent.GetLevelUpPoints` _returnvalue "CraftingSpeedMultiplier" false))) false false true 30.0)))))

(fn `Debug`
  (params (String :type String) (PrintString :type Boolean) (Notification :type Boolean) (toServerLog :type Boolean) (DisplayTime :type "Float (double-precision)"))
  (bind _returnvalue (`GameplayStatics.GetGameMode`))
  (bind _returnvalue_2 (`KismetStringLibrary.Concat_StrStr` (`KismetMathLibrary.SelectString` "NCQuetzal: Server: " "NCQuetzal: Client: " (`self.HasAuthority`)) String))
  (if PrintString
    (`KismetSystemLibrary.PrintString` _returnvalue_2))
  (`/Engine/EditorBlueprintResources/StandardMacros.IsValid` _returnvalue
    (:`Is Valid`
      (bind _asshootergamemode (cast `ShooterGameMode` _returnvalue))
      (if Notification
        (`|ExecutionSequence`
          (:`then_0`
            (`ShooterGameMode.SendServerNotification` _asshootergamemode _returnvalue_2 (struct :`R` 0.341845 :`G` 1.0 :`B` 0.32 :`A` 1.0) 1.0 DisplayTime null null -1 -1 false))
          (:`then_1`
            (if toServerLog :!label _label
              (`ShooterGameMode.PrintToServerGameLog` _asshootergamemode _returnvalue_2 true))))
        (else
          (goto _label))))
    (:`Is Not Valid`
      (bind _asshooterplayercontroller (cast `ShooterPlayerController` (`GameplayStatics.GetPlayerController` 0))
        (:`then`
          (`ShooterPlayerController.ClientServerNotification` _asshooterplayercontroller _returnvalue_2 (struct :`R` 1.0 :`A` 1.0) 1.0 DisplayTime null null))
        (:`CastFailed`
          (`KismetSystemLibrary.PrintString` "Controller Cast failed"))))))

(fn `UserConstructionScript`
  (`parent.UserConstructionScript`)
  (bind _returnvalue (`VictoryCore.ServerOctreeOverlapActorsClass` (`self.K2_GetWorld` self) (`self.K2_GetActorLocation` self) 100000.0 "DINOPAWNS" (`self.MyClass`)))
  (set `self.WildinArea` _returnvalue))
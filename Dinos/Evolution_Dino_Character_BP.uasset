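; Base dino character that evolves into another dino class once its inventory holds enough of a required item.
; On BeginPlay the server reads the required count from a game INI option, which can only raise the default.
; A Ctrl+X keybind checks the inventory, then the server, given a valid rider, increments the item stack by that count and multicasts a particle effect.
; It spawns the new dino at the same level, tames it to the rider's team and destroys itself.
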(event `self.ReceiveBeginPlay`
  ;[1 1 1] Get Required Kills ini
  (`KismetSystemLibrary.Delay` 0.2)
  (`/Engine/EditorBlueprintResources/ActorMacros.Switch Has Authority`
    (:`Authority`
      (bind _asshootergamemode (cast `ShooterGameMode` (`GameplayStatics.GetGameMode`)))
      (`|ExecutionSequence`
        (:`then_0`
          (bind _returnvalue (`ShooterGameMode.GetFloatOptionIni` _asshootergamemode (`self.Evolve_ini_SectionString`) (`self.Evolve_ini_OptionName`)))
          (if (<= _returnvalue (`self.NumberOfItemsRequiredToEvolve`))
            (set `self.NumberOfItemsRequiredToEvolve` (`self.NumberOfItemsRequiredToEvolve`))
            (else
              (set `self.NumberOfItemsRequiredToEvolve` _returnvalue))))))))

(event `EvolveItemCheck`
  (bind _allowevolution (`self.AllowEvolution`))
  ;[1 1 1] item check
  (bind _returnvalue (`PrimalInventoryComponent.GetItemTemplateQuantity` (`self.MyInventoryComponent`) (`self.EvolutionItemRequired`) null true false false))
  (if (>= (`KismetMathLibrary.Conv_IntToDouble` _returnvalue) (`self.NumberOfItemsRequiredToEvolve`))
    (if (not _allowevolution)
      (set `self.AllowEvolution` true))
    (elif _allowevolution
      (set `self.AllowEvolution` false))))

(event `EvolveDino`
  (params (Character :type "PrimalCharacter Object Reference"))
  (bind _rider (`self.Rider`))
  ;[1 1 1] Evolution
  (`/Engine/EditorBlueprintResources/ActorMacros.Switch Has Authority`
    (:`Authority`
      (`/Engine/EditorBlueprintResources/StandardMacros.IsValid` _rider
        (:`Is Valid`
          (bind _returnvalue (`self.GetOwnerController` _rider))
          (`PrimalInventoryComponent.BPIncrementItemTemplateQuantity` (`self.MyInventoryComponent`) (`self.EvolutionItemRequired`) (`KismetMathLibrary.FFloor` (`self.NumberOfItemsRequiredToEvolve`)) true false true false false false null false)
          (bind _returnvalue_2 (`PrimalCharacter.GetCharacterStatusComponent`))
          (`self.MC_Divine_Particles`)
          (`KismetSystemLibrary.Delay` (`self.EvolveParticleDelay`))
          (bind _returnvalue_3 (`PrimalDinoCharacter.SpawnDino` (`self.K2_GetWorld`) (`self.DinoToEvolve`) (`self.K2_GetActorLocation`) (struct) 1.0 0 false false 0 false 1.0 (`PrimalCharacterStatusComponent.GetCharacterLevel` _returnvalue_2)))
          (bind _asshooterplayercontroller (cast `ShooterPlayerController` _returnvalue))
          (`PrimalDinoCharacter.TameDino` _returnvalue_3 _asshooterplayercontroller true (`Actor.TargetingTeam` _asshooterplayercontroller) false false)
          (`self.SetActorHiddenInGame` true)
          (`self.SetActorEnableCollision` false)
          (`KismetSystemLibrary.Delay` 0.2)
          (`self.K2_DestroyActor`))))))

(event `ROS_ActiveEvolve`
  ;[1 1 1] Evolution Keybind
  (`self.EvolveItemCheck`)
  (if (`self.AllowEvolution`)
    (`self.EvolveDino` null)))

(event `Key|Ctrl+X`
  ;[1 1 1] Evolution Keybind
  (:`Pressed`
    (`self.ROS_ActiveEvolve`)))

(event `MC_Divine_Particles`
  ;[1 1 1] Particle
  (bind _returnvalue (`GameplayStatics.SpawnEmitterAttached` (`self.EvolveParticle`) (`self.Mesh`) (`self.EvolveParticleAttachPoint`) (`self.EvolveParticleLocation`) (`KismetMathLibrary.Conv_VectorToRotator` (`self.EvolveParticleRotation`)) "SnapToTarget" true true true))
  (`SceneComponent.SetRelativeScale3D` _returnvalue (`self.EvolveParticleSize`)))

(fn `UserConstructionScript`
  (`parent.UserConstructionScript`))
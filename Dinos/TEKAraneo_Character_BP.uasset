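; TEK Araneo creature Blueprint that culls excess wild, stasised spiders of its own class to limit local population.
; Construction reads an optional MaxSpiderCount INI override and snapshots same-class dinos within a large radius using an octree query.
; A server-side timer repeatedly pops the first entry, destroying it if untamed and stasised.
; Purging stops at Min(MaxWildCount/10, 1), so the threshold never exceeds one.
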(event `Purge`
  (bind _wildinarea (`self.WildinArea`))
  (bind _item (`KismetArrayLibrary.Array_Get` _wildinarea))
  (if (> (`KismetArrayLibrary.Array_Length` _wildinarea) (`KismetMathLibrary.Min` (/ (`self.MaxWildCount`) 10) 1))
    (bind _astekaraneo_character_bp_c (cast `/Dinos/TEKAraneo_Character_BP` _item)
      (:`then`
        (if (and (not (`self.BPIsTamed` _astekaraneo_character_bp_c)) (`Actor.bStasised` _astekaraneo_character_bp_c))
          (`/Engine/EditorBlueprintResources/StandardMacros.IsValid` _item
            (:`Is Valid`
              (`self.K2_DestroyActor` _item))
            (:`Is Not Valid`
              _)))
        (`KismetArrayLibrary.Array_Remove` _wildinarea))
      (:`CastFailed`
        _))
    (`KismetSystemLibrary.K2_SetTimer` null "Purge" 2.0)
    (else
      (`KismetSystemLibrary.K2_ClearTimer` null "Purge"))))

(event `self.ReceiveBeginPlay`
  (`KismetSystemLibrary.Delay` 0.2)
  (`/Engine/EditorBlueprintResources/ActorMacros.Switch Has Authority`
    (:`Authority`
      (`KismetSystemLibrary.K2_SetTimer` null "Purge" 2.0))))

(fn `UserConstructionScript`
  (`parent.UserConstructionScript`)
  (bind _asshootergamemode (cast `ShooterGameMode` (`GameplayStatics.GetGameMode`)))
  (bind _returnvalue (`ShooterGameMode.GetIntOptionIni` _asshootergamemode "AccessibleTEK" "MaxSpiderCount"))
  (set `self.MaxWildCount` (`KismetMathLibrary.SelectInt` _returnvalue (`self.MaxWildCount`) (> _returnvalue 0)))
  (bind _returnvalue_2 (`VictoryCore.ServerOctreeOverlapActorsClass` (`self.K2_GetWorld` self) (`self.K2_GetActorLocation` self) 50000.0 "DINOPAWNS" (`self.MyClass`)))
  (set `self.WildinArea` _returnvalue_2))